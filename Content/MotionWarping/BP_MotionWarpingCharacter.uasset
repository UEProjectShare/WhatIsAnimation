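; Test character Blueprint that demonstrates Motion Warping with a vault animation.
; Pressing the 1 key takes the first TargetPoint actor found in the level and registers its transform as the "TestWarp" warp target on the MotionWarping component.
; It then plays the VaultOver montage on the mesh so its warp windows can align the motion to that target.
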(event `self.ReceiveBeginPlay`
  (`parent.ReceiveBeginPlay`))

(event `Key|One`
  (params (Key :type "Key Structure"))
  (:`Pressed`
    (bind _outactors (`GameplayStatics.GetAllActorsOfClass` "/Script/Engine.TargetPoint"))
    (`MotionWarpingComponent.AddOrUpdateWarpTargetFromTransform` (`self.MotionWarping`) "TestWarp" (`self.GetTransform` (`|GetArrayItem` _outactors)))
    (`|PlayMontage` (`self.Mesh`) "/Game/MotionWarping/VaultOver_Montage.VaultOver_Montage")))

(fn `UserConstructionScript`
  (`parent.UserConstructionScript`))